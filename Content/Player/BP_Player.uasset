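; BP_Player is the player character Blueprint, a flipbook sprite driven by Enhanced Input for movement, jumping, turning and a timed "Squart" move.
; Movement follows controller yaw and switches run and idle flipbooks, while turn inputs snap sprite and spring arm to fixed opposite rotations.
; Squart requires active move input, temporarily swaps walk speed and flipbook, then restores the animation by velocity and starts a cooldown.
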(event Input|EnhancedActionEvents|EnhancedInputActionIA_Move
  (params (ActionValue :type Vector%202D%20Structure) (ElapsedSeconds :type Float%20%28double-precision%29) (TriggeredSeconds :type Float%20%28double-precision%29) (InputAction :type Input%20Action%20Object%20Reference :default "/Game/Input/Action/IA_Move.IA_Move"))
  (bind _returnvalue (Game|GetPlayerController 0))
  (bind _returnvalue_2 (Pawn|GetControlRotation _returnvalue :!class /Script/Engine.Controller))
  (:Triggered
    (Pawn|Input|AddMovementInput (Math|Vector|GetRightVector (Math|Rotator|MakeRotator (.roll _returnvalue_2) 0.0 (.yaw _returnvalue_2))) (.x ActionValue) false)
    (Pawn|Input|AddMovementInput (Math|Vector|GetForwardVector (Math|Rotator|MakeRotator 0.0 0.0 (.yaw (Pawn|GetControlRotation (Game|GetPlayerController 0) :!class /Script/Engine.Controller)))) (.y ActionValue) false))
  (:Started
    (Sprite|SetFlipbook (Variables|Default|GetSprite) "/Game/Player/Animation/Ani_Chara_Run.Ani_Chara_Run")
    (Variables|Default|SetCouldSquart? true))
  (:Completed
    (Sprite|SetFlipbook (Variables|Default|GetSprite) "/Game/Player/Animation/Ani_Chara_Wait.Ani_Chara_Wait")
    (Variables|Default|SetCouldSquart? false)))

(event Input|EnhancedActionEvents|EnhancedInputActionIA_TurnLeft
  (params (ActionValue :type Boolean) (ElapsedSeconds :type Float%20%28double-precision%29) (TriggeredSeconds :type Float%20%28double-precision%29) (InputAction :type Input%20Action%20Object%20Reference :default "/Game/Input/Action/IA_TurnLeft.IA_TurnLeft"))
  (:Started
    (Transformation|SetRelativeRotation (Variables|Default|GetSprite) "0.000000,90.000000,0.000000" false false)
    (Transformation|SetRelativeRotation (Variables|Default|GetSpringArm) "0.000000,90.000000,0.000000" false false)))

(event Input|EnhancedActionEvents|EnhancedInputActionIA_TurnRight
  (params (ActionValue :type Boolean) (ElapsedSeconds :type Float%20%28double-precision%29) (TriggeredSeconds :type Float%20%28double-precision%29) (InputAction :type Input%20Action%20Object%20Reference :default "/Game/Input/Action/IA_TurnRight.IA_TurnRight"))
  (:Started
    (Transformation|SetRelativeRotation (Variables|Default|GetSprite) "0.000000,-90.000000,0.000000" false false)
    (Transformation|SetRelativeRotation (Variables|Default|GetSpringArm) "0.000000,-90.000000,0.000000" false false)))

(event Input|EnhancedActionEvents|EnhancedInputActionIA_Jump
  (params (ActionValue :type Boolean) (ElapsedSeconds :type Float%20%28double-precision%29) (TriggeredSeconds :type Float%20%28double-precision%29) (InputAction :type Input%20Action%20Object%20Reference :default "/Game/Input/Action/IA_Jump.IA_Jump"))
  (:Triggered
    (Character|Jump))
  (:Completed
    (Character|StopJumping)))

(event Input|EnhancedActionEvents|EnhancedInputActionIA_Squart
  (params (ActionValue :type Boolean) (ElapsedSeconds :type Float%20%28double-precision%29) (TriggeredSeconds :type Float%20%28double-precision%29) (InputAction :type Input%20Action%20Object%20Reference :default "/Game/Input/Action/IA_Squart.IA_Squart"))
  (:Triggered
    (if (and (Variables|Default|GetCouldSquart?) (not (Variables|Default|GetIsInSquartCD?)))
      (Utilities|FlowControl|Sequence
        (:then_0
          (Variables|/Script/Engine.CharacterMovementComponent|SetMaxWalkSpeed (Variables|Character|GetCharacterMovement) (Variables|Default|GetSquartSpeed))
          (Utilities|FlowControl|Delay (Variables|Default|GetSquartTime))
          (Variables|/Script/Engine.CharacterMovementComponent|SetMaxWalkSpeed (Variables|Character|GetCharacterMovement) (Variables|Default|GetRunSpeed))
          (Variables|Default|SetIsInSquartCD? true)
          (Utilities|FlowControl|Delay (Variables|Default|GetSquartCD))
          (Variables|Default|SetIsInSquartCD? false))
        (:then_1
          (Sprite|SetFlipbook (Variables|Default|GetSprite) "/Game/Player/Animation/Ani_Chara_Squart.Ani_Chara_Squart")
          (Utilities|FlowControl|Delay (Variables|Default|GetSquartTime))
          (Sprite|SetFlipbook (Variables|Default|GetSprite) (select (<= 1e+01 (Math|Vector|VectorLength (Transformation|GetVelocity))) "/Game/Player/Animation/Ani_Chara_Run.Ani_Chara_Run" "/Game/Player/Animation/Ani_Chara_Wait.Ani_Chara_Wait")))))))

(fn ConstructionScript)