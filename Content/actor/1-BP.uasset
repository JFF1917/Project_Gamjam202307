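; An actor blueprint that starts and ends a dialogue when the player character enters and leaves its Box trigger, likely an NPC.
; Both overlap events pass the other actor through macro "1", which continues only if it casts to BP_ThirdPersonCharacter.
; On entry it calls 开始对话 (start dialogue) on 对话组件 (dialogue component) and hides the Name component.
; On exit it calls 结束对话 (end dialogue) and shows Name again.
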(event OnComponentBeginOverlap(Box)
  (params (OverlappedComponent :type Primitive%20Component%20Object%20Reference) (OtherActor :type Actor%20Object%20Reference) (OtherComp :type Primitive%20Component%20Object%20Reference) (OtherBodyIndex :type Integer) (bFromSweep :type Boolean) (SweepResult :type Hit%20Result%20Structure%20%28by%20ref%29))
  (Utilities|1 OtherActor
    (:NewParam3
      (Default|开始对话 (Variables|组件|Get对话组件))
      (Rendering|SetVisibility (Variables|组件|Getname) false false))))

(event OnComponentEndOverlap(Box)
  (params (OverlappedComponent :type Primitive%20Component%20Object%20Reference) (OtherActor :type Actor%20Object%20Reference) (OtherComp :type Primitive%20Component%20Object%20Reference) (OtherBodyIndex :type Integer))
  (Utilities|1 OtherActor
    (:NewParam3
      (Default|结束对话 (Variables|组件|Get对话组件))
      (Rendering|SetVisibility (Variables|组件|Getname) true false))))

(fn ConstructionScript)