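; BP_Item is an interactable item actor that adds an entry to the player's item array when interacted with.
; Overlapping its InteractionBox shows a widget, sets CouldInteract and sets the player's InteractType to "Item"; ending overlap hides the widget and clears the flag.
; Interact appends the player's own ItemRowName to ItemArray.
; Overlap events don't check the overlapping actor and always target player 0.
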(event OnComponentBeginOverlap(InteractionBox)
  (params (OverlappedComponent :type Primitive%20Component%20Object%20Reference) (OtherActor :type Actor%20Object%20Reference) (OtherComp :type Primitive%20Component%20Object%20Reference) (OtherBodyIndex :type Integer) (bFromSweep :type Boolean) (SweepResult :type Hit%20Result%20Structure%20%28by%20ref%29))
  (Rendering|SetVisibility (Variables|Default|GetWidget) true true)
  (Variables|Default|SetCouldInteract? true)
  (bind _asbp_player (Utilities|Casting|CastToBP_Player (Game|GetPlayerCharacter 0)))
  (Variables|/Game/Player/BP_Player.BP_Player_C|SetInteractType _asbp_player "Item"))

(event OnComponentEndOverlap(InteractionBox)
  (params (OverlappedComponent :type Primitive%20Component%20Object%20Reference) (OtherActor :type Actor%20Object%20Reference) (OtherComp :type Primitive%20Component%20Object%20Reference) (OtherBodyIndex :type Integer))
  (Rendering|SetVisibility (Variables|Default|GetWidget) false true)
  (Variables|Default|SetCouldInteract? false))

(event Custom|Interact
  (bind _asbp_player (Utilities|Casting|CastToBP_Player (Game|GetPlayerCharacter 0)))
  (Utilities|Array|Add (Variables|/Game/Player/BP_Player.BP_Player_C|GetItemArray _asbp_player) (Variables|/Game/Player/BP_Player.BP_Player_C|GetItemRowName _asbp_player)))

(fn ConstructionScript)

(fn Fun)