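; BP_NPC_RedRock_1 is an NPC blueprint that picks which dialog the player gets based on items they carry.
; When its InteractionBox is overlapped, it caches the player character and copies its ItemArray.
; Nested checks for certain cloth, hair and book items then write one of three DialogID values onto the player.
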(event OnComponentBeginOverlap(InteractionBox)
  (params (OverlappedComponent :type Primitive%20Component%20Object%20Reference) (OtherActor :type Actor%20Object%20Reference) (OtherComp :type Primitive%20Component%20Object%20Reference) (OtherBodyIndex :type Integer) (bFromSweep :type Boolean) (SweepResult :type Hit%20Result%20Structure%20%28by%20ref%29))
  (Utilities|FlowControl|Sequence
    (:then_0
      (bind _asbp_player (Utilities|Casting|CastToBP_Player (Game|GetPlayerCharacter 0)))
      (Variables|Default|SetBP_Player_Ins _asbp_player)
      (Variables|Default|SetItem%20Array (Variables|/Game/Player/BP_Player.BP_Player_C|GetItemArray (Variables|Default|GetBP_Player_Ins))))
    (:then_1
      (if (or (Utilities|Array|ContainsItem (Variables|Default|GetItem%20Array) "Cloth_2") (Utilities|Array|ContainsItem (Variables|Default|GetItem%20Array) "Cloth_3"))
        (if (or (Utilities|Array|ContainsItem (Variables|Default|GetItem%20Array) "Hair_1") (Utilities|Array|ContainsItem (Variables|Default|GetItem%20Array) "Hair_3"))
          (if (Utilities|Array|ContainsItem (Variables|Default|GetItem%20Array) "Book_2")
            (Variables|/Game/Player/BP_Player.BP_Player_C|SetDialogID (Variables|Default|GetBP_Player_Ins) "401")
            (else
              (Variables|/Game/Player/BP_Player.BP_Player_C|SetDialogID (Variables|Default|GetBP_Player_Ins) "501")))
          (else
            (Variables|/Game/Player/BP_Player.BP_Player_C|SetDialogID (Variables|Default|GetBP_Player_Ins) "601" :!label _label)))
        (else
          (goto _label))))))

(fn ConstructionScript
  (|CallParentFunction))