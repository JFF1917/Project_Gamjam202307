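; NPC actor that the player can interact with when inside its interaction box, as the entry point for dialog.
; Overlap begin shows the widget, sets CouldInteract and tags the player's InteractType as "NPC"; overlap end hides it and clears only CouldInteract.
; Interact removes the IMC_PlayerControl input mapping, then reads the DT_Dialog row keyed by the player's DialogID, though nothing uses that row yet.
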(event OnComponentBeginOverlap(InteractionBox)
  (params (OverlappedComponent :type Primitive%20Component%20Object%20Reference) (OtherActor :type Actor%20Object%20Reference) (OtherComp :type Primitive%20Component%20Object%20Reference) (OtherBodyIndex :type Integer) (bFromSweep :type Boolean) (SweepResult :type Hit%20Result%20Structure%20%28by%20ref%29))
  (Rendering|SetVisibility (Variables|Default|GetWidget) true true)
  (Variables|Default|SetCouldInteract? true)
  (bind _asbp_player (Utilities|Casting|CastToBP_Player (Game|GetPlayerCharacter 0)))
  (Variables|/Game/Player/BP_Player.BP_Player_C|SetInteractType _asbp_player "NPC"))

(event OnComponentEndOverlap(InteractionBox)
  (params (OverlappedComponent :type Primitive%20Component%20Object%20Reference) (OtherActor :type Actor%20Object%20Reference) (OtherComp :type Primitive%20Component%20Object%20Reference) (OtherBodyIndex :type Integer))
  (Rendering|SetVisibility (Variables|Default|GetWidget) false true)
  (Variables|Default|SetCouldInteract? false))

(event Custom|Interact
  (Utilities|FlowControl|Sequence
    (:then_0
      (bind _as玩家控制器 (Utilities|Casting|CastToPlayerController (Game|GetPlayerController 0)))
      (Utilities|IsValid (PlayerController|LocalPlayerSubsystems|GetEnhancedInputLocalPlayerSubsystem _as玩家控制器)
        (:Is%20Valid
          (Input|RemoveMappingContext (PlayerController|LocalPlayerSubsystems|GetEnhancedInputLocalPlayerSubsystem _as玩家控制器) "/Game/Input/IMC_PlayerControl.IMC_PlayerControl" "(bIgnoreAllPressedKeysUntilRelease=True,bForceImmediately=False)"))))
    (:then_1
      (bind _asbp_player (Utilities|Casting|CastToBP_Player (Game|GetPlayerCharacter 0)))
      (bind _returnvalue (Utilities|GetDataTableRow "/Game/DataTable/DT_Dialog.DT_Dialog" (Variables|/Game/Player/BP_Player.BP_Player_C|GetDialogID _asbp_player))))))

(fn ConstructionScript)

(fn Fun)